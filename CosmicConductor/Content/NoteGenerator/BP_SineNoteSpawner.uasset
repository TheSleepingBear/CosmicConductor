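; BP_SineNoteSpawner is a note generator that spawns BP_SplineNotes actors at its own location, one per second, up to MaxSpawn.
; A looping timer started on BeginPlay calls SpawnTimer, which checks and increments SpawnCount.
; Each note receives the spawner's X and Y forward motion, Amplitude and Period at spawn, so its motion is configured per spawner.
; The timer keeps running after the cap is reached.
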(event `self.ReceiveBeginPlay`
  (`KismetSystemLibrary.K2_SetTimer` null "SpawnTimer" 1.0 true))

(fn `SpawnTimer`
  (if (< (`self.SpawnCount`) (`self.MaxSpawn`))
    (`|SpawnActorFromClass` "/Game/NoteGenerator/BP_SplineNotes.BP_SplineNotes_C" (`KismetMathLibrary.MakeTransform` (`self.K2_GetActorLocation`) (struct)) "Undefined" "OverrideRootScale" null (`self.Xmove`) (`self.Ymove`) (`self.Amplitude`) (`self.Period`))
    (`/Engine/EditorBlueprintResources/StandardMacros.IncrementInt` (`self.SpawnCount`))))

(fn `UserConstructionScript`)