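; BP_StaticSpline is a spawner actor that lays out a row of BP_StaticNote actors in a sine wave when play begins.
; BeginPlay calls SpawnWave, which loops up to MaxCount, stepping each note back along world X from the actor and setting its height with a sine of the index.
; Amplitude multiplies the whole height, including the actor's own Z, and the graph uses no spline component despite the name.
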(event `SpawnWave`
  (bind (_returnvalue_x _returnvalue_y _returnvalue_z) (`KismetMathLibrary.BreakVector` (`self.K2_GetActorLocation`)))
  (for _index (range 1 (+ (`self.MaxCount`) 1))
    (`|SpawnActorFromClass` "/Game/NoteGenerator/BP_StaticNote.BP_StaticNote_C" (`KismetMathLibrary.MakeTransform` (`KismetMathLibrary.MakeVector` (- _returnvalue_x (* _index 100.0)) _returnvalue_y (* (`self.Amplitude`) (+ _returnvalue_z (* (`KismetMathLibrary.DegSin` (* _index 30.0)) 200.0))))) "Undefined" "OverrideRootScale")))

(event `self.ReceiveBeginPlay`
  (`self.SpawnWave`))

(fn `UserConstructionScript`)